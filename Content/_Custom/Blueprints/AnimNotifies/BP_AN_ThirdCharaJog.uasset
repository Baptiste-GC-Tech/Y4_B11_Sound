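; Anim notify that plays footstep sounds for the third-person character's jog, based on the surface underfoot.
; A short Visibility line trace runs down from the mesh owner's location and switches on the hit physical material's object name.
; Cloth and Netherite materials each select their own sound cue, played as non-spatial 2D audio.
; Any other material clears the sound and plays nothing.
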(fn `Received_Notify`
  (params (MeshComp :type "SkeletalMeshComponent Object Reference") (Animation :type "AnimSequenceBase Object Reference") (EventReference :type "AnimNotifyEventReference Structure (by ref)"))
  (returns (ReturnValue :type Boolean))
  (locals (SoundToPlay :type "SoundBase Object Reference"))
  (bind _returnvalue (`Actor.K2_GetActorLocation` (`ActorComponent.GetOwner` MeshComp)))
  (bind _outhit (`KismetSystemLibrary.LineTraceSingle` _returnvalue (+ _returnvalue (* (`KismetMathLibrary.Vector_Down`) 100.0)) "TraceTypeQuery1"))
  (bind (_bblockinghit _binitialoverlap _time _distance _location _impactpoint _normal _impactnormal _physmat) (`GameplayStatics.BreakHitResult` _outhit))
  (if _bblockinghit
    (switch `string` (`KismetSystemLibrary.GetObjectName` _physmat)
      (:`Default`
        (set `local.SoundToPlay` null)
        (return false))
      (:`PM_Cloth`
        (set `local.SoundToPlay` "/Game/_Custom/Sounds/SC_ClothFootstep.SC_ClothFootstep"))
      (:`PM_Netherite`
        (set `local.SoundToPlay` "/Game/_Custom/Sounds/SC_NetheriteFootstep.SC_NetheriteFootstep")))
    (`GameplayStatics.PlaySound2D` (`local.SoundToPlay`) 1.0 1.0 0.0 null null)
    (return true)))