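; BP_MenacingEvilFoe is a foe actor that drives an ambient sound crossfade by its proximity to the player.
; Each Tick, PrepareCrossfaceValue measures distance to player 0, assuming single-player, and AmbientSound receives the result as the "CrossfadeValue" parameter.
; The value clamps at two thresholds; between them it falls linearly with distance over NoEffectThreshold alone, so it jumps at MaxEffectThreshold.
; Distance prints on screen for debugging.
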(event `self.ReceiveBeginPlay`)

(event `self.ReceiveTick`
  (params (DeltaSeconds :type "Float (single-precision)"))
  (`self.PrepareCrossfaceValue`)
  (`AudioParameterControllerInterface.SetFloatParameter` (`AmbientSound.AudioComponent` (`self.AmbientSound`)) "CrossfadeValue" (`self.CrossfadeValue`)))

(fn `PrepareCrossfaceValue`
  (bind _returnvalue (`KismetMathLibrary.Vector_Distance` (`self.K2_GetActorLocation`) (`self.K2_GetActorLocation` (`GameplayStatics.GetPlayerCharacter` 0))))
  (`KismetSystemLibrary.PrintString` (`KismetStringLibrary.Conv_DoubleToString` _returnvalue) true false (struct :`G` 0.66 :`B` 1.0 :`A` 1.0) 0.0 "Dist")
  (if (>= _returnvalue (`self.NoEffectThreshold`))
    (set `self.CrossfadeValue` 0.0)
    (elif (<= _returnvalue (`self.MaxEffectThreshold`))
      (set `self.CrossfadeValue` 1.0)
      (else
        (set `self.CrossfadeValue` (+ (* (/ _returnvalue (`self.NoEffectThreshold`)) -1.0) 1.0)))))
  (return))

(fn `UserConstructionScript`)