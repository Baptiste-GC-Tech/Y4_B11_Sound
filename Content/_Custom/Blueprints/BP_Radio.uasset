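; Interactable radio actor that lets the player tune between music stations by frequency.
; Entering its sphere shows an interaction prompt, and interacting opens a frequency picker whose changes update a camera-facing world widget.
; All station tracks spawn muted at BeginPlay, then each volume fades by its distance from the tuned frequency within a tolerance.
; The tuned and nearest station frequencies also drive RadioAudio parameters; an unused single-MetaSound wave-swapping attempt remains.
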(event `CloseWindow`
  (bind _returnvalue (`GameplayStatics.GetPlayerController` 0))
  (bind _returnvalue_2 (`GameplayStatics.GetPlayerController` 0))
  (`Widget.RemoveFromParent` (`self.FrenquencyChoiceUI`))
  (set `PlayerController.bShowMouseCursor` false _returnvalue)
  (`WidgetBlueprintLibrary.SetInputMode_GameOnly` _returnvalue)
  (`EnhancedInputSubsystemInterface.AddMappingContext` (pcsubsystem `EnhancedInputLocalPlayerSubsystem` _returnvalue_2) "/Game/Input/IMC_Interact.IMC_Interact" 0 (struct))
  (`self.EnableInput` _returnvalue_2)
  (bind _returnvalue_3 (`|CreateWidget` "/Game/_Custom/UI/WB_Interaction.WB_Interaction_C" (`GameplayStatics.GetPlayerController` 0)))
  (bind _output_get (set `self.InteractionUI` _returnvalue_3))
  (`UserWidget.AddToViewport` _output_get 0))

(event `EnhancedInput|/Game/Input/Actions/IA_Interact`
  (params (ActionValue :type Boolean) (ElapsedSeconds :type "Float (double-precision)") (TriggeredSeconds :type "Float (double-precision)") (InputAction :type "InputAction Object Reference" :default "/Game/Input/Actions/IA_Interact.IA_Interact"))
  (bind _returnvalue (`GameplayStatics.GetPlayerController` 0))
  (:`Started`
    (bind _returnvalue_2 (`|CreateWidget` "/Game/_Custom/UI/WB_FrequencyChoice.WB_FrequencyChoice_C" _returnvalue self))
    (`UserWidget.AddToViewport` _returnvalue_2 0)
    (`WidgetBlueprintLibrary.SetInputMode_UIOnlyEx` _returnvalue _returnvalue_2)
    (bind _output_get (set `self.FrenquencyChoiceUI` _returnvalue_2))
    (add `/Game/_Custom/UI/WB_FrequencyChoice.ValueChanged` _output_get (delegate `SetFrequency`))
    (add `/Game/_Custom/UI/WB_FrequencyChoice.CloseWindow` _returnvalue_2 (delegate `CloseWindow`))
    (set `PlayerController.bShowMouseCursor` true (`GameplayStatics.GetPlayerController` 0))
    (`Widget.RemoveFromParent` (`self.InteractionUI`))))

(event `SetFrequency`
  (params (Frequency :type "Float (double-precision)"))
  (bind _returnvalue (`GameplayStatics.GetPlayerController` 0))
  (bind _radioaudio (`self.RadioAudio`))
  (set `self.CurrentFrequency` Frequency)
  (set `self.LowestDeltaFrequency` 9999.0)
  (bind (_keypin _valuepin) (`|MapForEach` (`self.SpawnedMusicComponents`))
    (:`then`
      (bind _returnvalue_2 (`KismetMathLibrary.Abs` (- _keypin (`self.CurrentFrequency`))))
      (if (< _returnvalue_2 (`self.LowestDeltaFrequency`))
        (set `self.CurrentMusicFrequency` _keypin)
        (set `self.LowestDeltaFrequency` _returnvalue_2))
      (`AudioComponent.SetVolumeMultiplier` _valuepin (`KismetMathLibrary.MapRangeClamped` _returnvalue_2 0.0 (`self.FrequencyTolerance`) 1.0)))
    (:`CompletedPin`
      (`AudioParameterControllerInterface.SetFloatParameter` _radioaudio "Frequency" (`self.CurrentFrequency`))
      (`AudioParameterControllerInterface.SetFloatParameter` _radioaudio "FrequencyMusic" (`self.CurrentMusicFrequency`))
      (bind _aswb_radio (cast `/Game/_Custom/UI/WB_Radio` (`WidgetComponent.GetUserWidgetObject` (`self.RadioUI`))))
      (`/Game/_Custom/UI/WB_Radio.SetFrequency` _aswb_radio (`self.CurrentFrequency`))
      (message `EnhancedInputSubsystemInterface.RemoveMappingContext` (pcsubsystem `EnhancedInputLocalPlayerSubsystem` _returnvalue) "/Game/Input/IMC_Interact.IMC_Interact" (struct))
      (`self.DisableInput` _returnvalue))))

(event `self.ReceiveTick`
  (params (DeltaSeconds :type "Float (single-precision)"))
  (bind _radioui (`self.RadioUI`))
  (`SceneComponent.K2_SetWorldRotation` _radioui (`KismetMathLibrary.FindLookAtRotation` (`SceneComponent.K2_GetComponentLocation` _radioui) (`PlayerCameraManager.GetCameraLocation` (`GameplayStatics.GetPlayerCameraManager` 0))) false false))

(event `self.Sphere.OnComponentBeginOverlap`
  (params (OverlappedComponent :type "PrimitiveComponent Object Reference") (OtherActor :type "Actor Object Reference") (OtherComp :type "PrimitiveComponent Object Reference") (OtherBodyIndex :type Integer) (bFromSweep :type Boolean) (SweepResult :type "HitResult Structure (by ref)"))
  (bind _returnvalue (`GameplayStatics.GetPlayerController` 0))
  (cast `/Game/ThirdPerson/Blueprints/BP_ThirdPersonCharacter` OtherActor)
  (`EnhancedInputSubsystemInterface.AddMappingContext` (pcsubsystem `EnhancedInputLocalPlayerSubsystem` _returnvalue) "/Game/Input/IMC_Interact.IMC_Interact" 0 (struct))
  (`self.EnableInput` _returnvalue)
  (bind _returnvalue_2 (`|CreateWidget` "/Game/_Custom/UI/WB_Interaction.WB_Interaction_C" (`GameplayStatics.GetPlayerController` 0)))
  (bind _output_get (set `self.InteractionUI` _returnvalue_2))
  (`UserWidget.AddToViewport` _output_get 0))

(event `self.Sphere.OnComponentEndOverlap`
  (params (OverlappedComponent :type "PrimitiveComponent Object Reference") (OtherActor :type "Actor Object Reference") (OtherComp :type "PrimitiveComponent Object Reference") (OtherBodyIndex :type Integer))
  (bind _returnvalue (`GameplayStatics.GetPlayerController` 0))
  (cast `/Game/ThirdPerson/Blueprints/BP_ThirdPersonCharacter` OtherActor)
  (`EnhancedInputSubsystemInterface.RemoveMappingContext` (pcsubsystem `EnhancedInputLocalPlayerSubsystem` _returnvalue) null (struct))
  (`self.DisableInput` _returnvalue)
  (`Widget.RemoveFromParent` (`self.InteractionUI`)))

(event `self.ReceiveBeginPlay`
  (bind (_keypin _valuepin) (`|MapForEach` (`self.MusicMap`))
    (:`then`
      (bind _returnvalue (`GameplayStatics.SpawnSoundAttached` _valuepin (`self.RadioUI`) "None" (0.0 0.0 0.0) (struct) "KeepRelativeOffset" false 1.0 1.0 0.0 "/Game/_Custom/Sounds/SA_Radio.SA_Radio" null))
      (`AudioComponent.SetVolumeMultiplier` _returnvalue 0.0)
      (`BlueprintMapLibrary.Map_Add` (`self.SpawnedMusicComponents`) _keypin _returnvalue))))

(fn `UserConstructionScript`)